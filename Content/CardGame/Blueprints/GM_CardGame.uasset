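; Card game mode that seats joining players, numbers them and runs turn order.
; New players get a spawned, possessed BP_PlayerPawn, a recorded name and number, and turn-based match interface registration; FindPlayerStart picks seats by player number.
; Turns cycle through controllers by index, wrapping to player one, with start and end messages sent to the active controller.
; Match start waits on the AllReady flag.
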(event `self.HandleStartingNewPlayer`
  (params (NewPlayer :type "PlayerController Object Reference"))
  ;[1 1 1] When Player Init Spawning Into Level Assign Number
  (`/Engine/EditorBlueprintResources/StandardMacros.IsValid` NewPlayer
    (:`Is Valid`
      (bind _result (`/Engine/EditorBlueprintResources/StandardMacros.IncrementInt` (`self.Number Of Players`))
        (:`  `
          (bind _returnvalue (`|SpawnActorFromClass` "/Game/CardGame/Blueprints/BP_PlayerPawn.BP_PlayerPawn_C" (`self.GetTransform` (`|GetArrayItem` (`self.Out Actors`) _result)) "AdjustIfPossibleButAlwaysSpawn" "OverrideRootScale" null null))
          (`Controller.Possess` NewPlayer _returnvalue)
          (bind _aspc_player (cast `/Game/CardGame/Blueprints/PC_Player` NewPlayer)
            (:`then`
              (`KismetArrayLibrary.Array_Add` (`self.Player Names`) (`/Game/CardGame/Blueprints/PC_Player.Player Name` _aspc_player))
              (bind _output_get (set `self.Number Of Players` (`self.Number Of Players`)))
              (set `/Game/CardGame/Blueprints/PC_Player.Player Number` _output_get _aspc_player)
              ;[1 1 1] Register Turn-Based Interface
              (`TurnBasedBlueprintLibrary.RegisterTurnBasedMatchInterfaceObject` NewPlayer self))
            (:`CastFailed`
              ;[1 1 1] Event Error On Assign Number To Player At Spawn
              (`KismetSystemLibrary.PrintString` "Initializing New Player Set Up Error, Could Not Cast In Gamemode" true true (struct :`R` 1.0 :`G` 0.036769 :`A` 1.0) 15.0))))))))

(event `Start Current Active Player Turn`
  ;[1 1 1] Starts Next Active Player Turn, If First Round Choose First Player
  (bind _result (`/Engine/EditorBlueprintResources/StandardMacros.IncrementInt` (`self.Current Active Player Turn`))
    (:`  `
      (if (> _result (`self.Number Of Players`))
        (set `self.Current Active Player Turn` 1))
      (message `/Game/CardGame/Blueprints/BPI_PlayerController.Start Player Turn` (`GameplayStatics.GetPlayerController` (- (`self.Current Active Player Turn`) 1))))))

(event `End Active Player Turn`
  ;[1 1 1] End Turn For Current Player
  (message `/Game/CardGame/Blueprints/BPI_PlayerController.End Player Turn` (`GameplayStatics.GetPlayerController` (- (`self.Current Active Player Turn`) 1)))
  (`self.Start Current Active Player Turn`))

(fn `FindPlayerStart`
  (params (Player :type "Controller Object Reference") (IncomingName :type String))
  (returns (ReturnValue :type "Actor Object Reference"))
  ;[1 1 1] Choose Player Seat Based On Assigned Player Number
  (bind _aspc_player (cast `/Game/CardGame/Blueprints/PC_Player` Player)
    (:`then`
      (set `/Game/CardGame/Blueprints/PC_Player.Player Name` IncomingName _aspc_player)
      (bind _outactors (`GameplayStatics.GetAllActorsOfClass` "/Script/Engine.PlayerStart"))
      (set `self.Out Actors` _outactors)
      (return (`|GetArrayItem` _outactors (`/Game/CardGame/Blueprints/PC_Player.Player Number` _aspc_player))))
    (:`CastFailed`
      ;[1 1 1] If Cast Error While Assigning Seats
      (`KismetSystemLibrary.PrintString` "Player Controller Failed To Cast To Get Player Index To Assign Seat" true true (struct :`R` 1.0 :`B` 0.979897 :`A` 1.0) 15.0))))

(fn `ReadyToStartMatch`
  (returns (ReturnValue :type Boolean))
  (return (== (`self.All Ready?`) true)))

(fn `UserConstructionScript`)