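; Game instance for the card game that handles multiplayer session hosting, browsing and joining.
; HostSever creates a session with the given player limit and LAN flag, then opens PlayingLevel as a listen server.
; FindServerList caches non-LAN search results in AllSessions, while JoinServer runs a fresh search and joins by index into those new results.
; Handled failures print an error and return to MainMenuLevel.
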(event `/Game/CardGame/Blueprints/BPI_CardGame.Host Sever`
  (params (`Max Players` :type Integer) (`LAN?` :type Boolean))
  ;[1 1 1] Hosting Session
  (`CreateSessionCallbackProxy.CreateSession` (`GameplayStatics.GetPlayerController` 0) `Max Players` `LAN?`
    (:`OnSuccess`
      (`GameplayStatics.OpenLevel` "PlayingLevel" true "listen"))
    (:`OnFailure`
      (`KismetSystemLibrary.PrintString` "Error Creating Host Session. Please Check Your Internet Connection And Try Again" true true (struct :`R` 0.144546 :`G` 1.0 :`A` 1.0) 10.0)
      (`GameplayStatics.OpenLevel` "MainMenuLevel"))))

(event `/Game/CardGame/Blueprints/BPI_CardGame.Find Server List`
  ;[1 1 1] Find Active Sessions
  (bind _results (`FindSessionsCallbackProxy.FindSessions` (`GameplayStatics.GetPlayerController` 0) 5)
    (:`OnSuccess`
      (set `self.All Sessions` _results))
    (:`OnFailure`
      (`KismetSystemLibrary.PrintString` "Error Getting Active Sessions. Please Check Your Internet Connection And Try Again" true true (struct :`R` 0.173022 :`G` 1.0 :`A` 1.0) 10.0)
      (`GameplayStatics.OpenLevel` "MainMenuLevel"))))

(event `/Game/CardGame/Blueprints/BPI_CardGame.JoinServer`
  (params (`Session INdex` :type Integer))
  ;[1 1 1] Join Selected Session
  (bind _results (`FindSessionsCallbackProxy.FindSessions` (`GameplayStatics.GetPlayerController` 0) 5)
    (:`OnSuccess`
      (`JoinSessionCallbackProxy.JoinSession` (`GameplayStatics.GetPlayerController` 0) (`|GetArrayItem` _results `Session INdex`)
        (:`OnFailure`
          (`KismetSystemLibrary.PrintString` "****Error Could Not Join Session.  Please Try Again***" true true (struct :`R` 0.173022 :`G` 1.0 :`A` 1.0) 10.0)
          (`GameplayStatics.OpenLevel` "MainMenuLevel"))))
    (:`OnFailure`
      (`KismetSystemLibrary.PrintString` "Error Getting Active Sessions. Please Check Your Internet Connection And Try Again" true true (struct :`R` 0.173022 :`G` 1.0 :`A` 1.0) 10.0)
      (`GameplayStatics.OpenLevel` "MainMenuLevel"))))