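; BP_PlayerPawn is a player pawn in the card game project, with free-look movement and a name label.
; Move axes add movement input along the camera's forward and right vectors, so forward movement follows the view pitch.
; Look axes add local pitch and yaw to the camera, clamping only each pitch delta, not the total angle.
; On BeginPlay, a text render component is set to the PlayerState's player name.
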(event `InputAxis|Move Forward`
  (params (AxisValue :type "Float (single-precision)"))
  (`self.AddMovementInput` (`SceneComponent.GetForwardVector` (`self.Camera`)) AxisValue))

(event `InputAxis|Move Right`
  (params (AxisValue :type "Float (single-precision)"))
  (`self.AddMovementInput` (`SceneComponent.GetRightVector` (`self.Camera`)) AxisValue))

(event `InputAxis|LookUp`
  (params (AxisValue :type "Float (single-precision)"))
  (`SceneComponent.K2_AddLocalRotation` (`self.Camera`) (`KismetMathLibrary.MakeRotator` 0.0 (`KismetMathLibrary.FClamp` AxisValue -60.0 60.0)) false false))

(event `InputAxis|Look RIght`
  (params (AxisValue :type "Float (single-precision)"))
  (`SceneComponent.K2_AddLocalRotation` (`self.Camera`) (`KismetMathLibrary.MakeRotator` 0.0 0.0 AxisValue) false false))

(event `self.ReceiveBeginPlay`
  (`TextRenderComponent.K2_SetText` (`self.TextRender`) (`|FormatText` "{Player}" (`PlayerState.GetPlayerName` (`self.PlayerState`)))))

(fn `UserConstructionScript`)